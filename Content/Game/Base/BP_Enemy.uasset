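; BP_Enemy is an enemy character Blueprint that awards experience to the player when it dies.
; It extends the parent's health-component death handler, then stops the AI controller's brain logic.
; If the damage instigator is a BP_Player, it adds its Exp value to that player's RPG stats component.
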(event `self.BndEvt__BPC_Health_K2Node_ComponentBoundEvent_0_ED_Death__DelegateSignature`
  (`parent.BndEvt__BPC_Health_K2Node_ComponentBoundEvent_0_ED_Death__DelegateSignature`)
  (`BrainComponent.StopLogic` (`AIController.BrainComponent` (`AIBlueprintHelperLibrary.GetAIController` self)) "i already die")
  (bind _asbp_player (cast `/Game/Game/Character/BP/BP_Player` (`self.DamageInstigated`)))
  (`/Game/Game/Character/BP/Components/BPC_RPGStats.AddExp` (`/Game/Game/Character/BP/BP_Player.BPC_RPGStats` _asbp_player) (`self.exp`)))

(fn `UserConstructionScript`
  (`parent.UserConstructionScript`))