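; Base character Blueprint that handles damage attribution, ragdoll death and movement input readouts.
; AnyDamage stores the instigating controller's pawn in DamageInstigated.
; The BPC_Health death event disables capsule collision and switches the mesh to physics simulation with collision.
; GetSpeedRM and GetTurnRM derive speed and turn values from the last movement input vector: its length, and its yaw offset from actor rotation scaled by that length.
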(event `self.ReceiveAnyDamage`
  (params (Damage :type "Float (single-precision)") (DamageType :type "DamageType Object Reference") (InstigatedBy :type "Controller Object Reference") (DamageCauser :type "Actor Object Reference"))
  (set `self.DamageInstigated` (`Controller.K2_GetPawn` InstigatedBy)))

(event `self.BPC_Health.ED_Death`
  (`PrimitiveComponent.SetCollisionEnabled` (`self.CapsuleComponent`) "NoCollision")
  (`PrimitiveComponent.SetSimulatePhysics` (`self.Mesh`) true)
  (`PrimitiveComponent.SetCollisionEnabled` (`self.Mesh`) "QueryAndPhysics"))

(fn `GetSpeedRM`
  (returns (speed :type "Float (double-precision)"))
  (return (`KismetMathLibrary.VSize` (`PawnMovementComponent.GetLastInputVector` (`self.CharacterMovement`)))))

(fn `GetTurnRM`
  (returns (turn :type "Float (double-precision)"))
  (bind _returnvalue (`PawnMovementComponent.GetLastInputVector` (`self.CharacterMovement`)))
  (bind (_returnvalue_roll _returnvalue_pitch _returnvalue_yaw) (`KismetMathLibrary.BreakRotator` (* (`KismetMathLibrary.NormalizedDeltaRotator` (`KismetMathLibrary.Conv_VectorToRotator` _returnvalue) (`self.K2_GetActorRotation`)) (`KismetMathLibrary.VSize` _returnvalue))))
  (return _returnvalue_yaw))

(fn `UserConstructionScript`)