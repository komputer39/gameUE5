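; Player character Blueprint that handles movement, jumping, mouse look and death.
; Axis inputs drive camera pitch and yaw, with movement relative to control yaw only, and GetSpeed and IsInAir expose movement state.
; The health component's death event disables capsule collision and turns the mesh into a physics ragdoll.
; Test hooks print health every tick and use Q and E to heal or damage the player.
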(event `InputAxis|LookUD`
  (params (AxisValue :type "Float (single-precision)"))
  ;[1 1 1] mouse
  (`self.AddControllerPitchInput` (* AxisValue -1.0)))

(event `InputAxis|lookLR`
  (params (AxisValue :type "Float (single-precision)"))
  ;[1 1 1] mouse
  (`self.AddControllerYawInput` AxisValue))

(event `InputAxis|Move forward`
  (params (AxisValue :type "Float (single-precision)"))
  (bind (_returnvalue_roll _returnvalue_pitch _returnvalue_yaw) (`KismetMathLibrary.BreakRotator` (`self.GetControlRotation`)))
  ;[1 1 1] controler
  (`self.AddMovementInput` (`KismetMathLibrary.GetForwardVector` (`KismetMathLibrary.MakeRotator` 0.0 0.0 _returnvalue_yaw)) AxisValue))

(event `InputAxis|strafe`
  (params (AxisValue :type "Float (single-precision)"))
  (bind (_returnvalue_roll _returnvalue_pitch _returnvalue_yaw) (`KismetMathLibrary.BreakRotator` (`self.GetControlRotation`)))
  ;[1 1 1] controler
  (`self.AddMovementInput` (`KismetMathLibrary.GetRightVector` (`KismetMathLibrary.MakeRotator` 0.0 0.0 _returnvalue_yaw)) AxisValue))

(event `InputAction|Jump`
  (params (Key :type "Key Structure"))
  ;[1 1 1] controler
  (:`Pressed`
    (`self.Jump`)))

(event `self.BPC_Health.ED_Death`
  ;[1 1 1] death
  (`PrimitiveComponent.SetCollisionEnabled` (`self.CapsuleComponent`) "NoCollision")
  (`PrimitiveComponent.SetSimulatePhysics` (`self.Mesh`) true)
  (`PrimitiveComponent.SetCollisionEnabled` (`self.Mesh`) "QueryAndPhysics"))

(event `self.ReceiveTick`
  (params (DeltaSeconds :type "Float (single-precision)"))
  ;[1 1 1] for tests damage
  (`KismetSystemLibrary.PrintString` (`KismetStringLibrary.Conv_DoubleToString` (`/Game/Game/Character/BP/Components/BPC_Health.GetHealth` (`self.BPC_Health`))) true true (struct :`R` 1.0 :`G` 0.1875 :`B` 0.1875 :`A` 1.0) 0.0))

(event `Key|Q`
  (params (Key :type "Key Structure"))
  ;[1 1 1] for tests damage
  (:`Pressed`
    (`/Game/Game/Character/BP/Components/BPC_Health.AddHealth` (`self.BPC_Health`) 5.0)))

(event `Key|E`
  (params (Key :type "Key Structure"))
  ;[1 1 1] for tests damage
  (:`Pressed`
    (`/Game/Game/Character/BP/Components/BPC_Health.Damage` (`self.BPC_Health`) 15.0)))

(fn `GetSpeed`
  (returns (speed :type "Float (double-precision)"))
  (return (`KismetMathLibrary.VSize` (`self.GetVelocity`))))

(fn `IsInAir`
  (returns (IsInAir :type Boolean))
  (return (`NavMovementComponent.IsFalling` (`self.CharacterMovement`))))

(fn `UserConstructionScript`)