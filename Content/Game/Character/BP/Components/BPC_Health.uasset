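; Health component that tracks a current and maximum health value for its owner, likely a character.
; It fills health on BeginPlay and exposes getters, capped healing, a full recovery and damage floored at zero.
; Event dispatchers report changes on start and healing, though not on damage.
; The death dispatcher sits behind a DoOnce that is never reset, so it fires only once, even after recovery.
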(event `self.ReceiveBeginPlay`
  (`self.Recovery`)
  (`self.ED_Change`))

(fn `AddHealth`
  (params (Add :type "Float (double-precision)"))
  (set `self.Health` (`KismetMathLibrary.FMin` (+ Add (`self.GetHealth`)) (`self.MaxHealth`)))
  (`self.ED_Change`))

(fn `Damage`
  (params (Damage :type "Float (double-precision)"))
  (bind _output_get (set `self.Health` (`KismetMathLibrary.FMax` (- (`self.Health`) (`local.Damage`)))))
  (if (== _output_get 0.0)
    (`/Engine/EditorBlueprintResources/StandardMacros.DoOnce` false
      (:`Completed`
        (`self.ED_Death`)))))

(fn `GetHealth`
  (returns (Health :type "Float (double-precision)"))
  (return (`self.Health`)))

(fn `GetPercentHealth`
  (returns (ReturnValue :type "Float (double-precision)"))
  (return (/ (`self.Health`) (`self.MaxHealth`))))

(fn `Recovery`
  (set `self.Health` (`self.MaxHealth`)))