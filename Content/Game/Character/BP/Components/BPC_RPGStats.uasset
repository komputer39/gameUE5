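; RPG stats component that tracks experience and level and derives damage, attack speed and critical chance from level.
; AddExp applies an experience multiplier, then UpdateLevel recomputes level from cumulative thresholds growing by 1000 per level and fires the level-up dispatcher on an increase.
; Stat getters compound base values by a per-level multiplier, capping all but damage.
; GetExpByLevel multiplies each step by zero, so it always returns zero.
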(fn `AddExp`
  (params (Add :type Integer))
  (set `self.Exp` (+ (* Add (`self.ExpMult`)) (`self.Exp`)))
  (`self.UpdateLevel`))

(fn `GetCriticalChance`
  (returns (CriticalCHance :type "Float (double-precision)"))
  (return (`self.GetStatByLevel` (`self.BaseCriticalChance`) (`self.IncBaseCriticalChanceByLevel`) (`self.MaxCriticalChance`))))

(fn `GetDamage`
  (returns (Damage :type "Float (double-precision)"))
  (return (`self.GetStatByLevel` (`self.BaseDamage`) (`self.IncDamageByLevel`) -1.0)))

(fn `GetExpByLevel`
  (params (ExampleLevel :type Integer))
  (returns (Exp :type Integer))
  (locals (L_level :type Integer) (L_Exp :type Integer))
  (for _index (range 1 ExampleLevel)
    (set `local.L_Exp` (+ (* _index 0) (`local.L_Exp`))))
  (return (`local.L_Exp`)))

(fn `GetLevel`
  (returns (Level :type Integer))
  (return (`self.Level`)))

(fn `GetLevelByExp`
  (params (ExampleExp :type Integer))
  (returns (Level :type Integer))
  (locals (L_level :type Integer) (L_Exp :type Integer))
  (while true
    (`/Engine/EditorBlueprintResources/StandardMacros.IncrementInt` (`local.L_level`)
      (:`  `
        (bind _output_get (set `local.L_Exp` (+ (`local.L_Exp`) (* (`local.L_level`) 1000))))
        (if (> _output_get (`local.ExampleExp`))
          (return (`local.L_level`)))))))

(fn `GetSpeedAttack`
  (returns (SpeedAttack :type "Float (double-precision)"))
  (return (`self.GetStatByLevel` (`self.BaseSpeedAttack`) (`self.IncSpeedAtackByLevel`) (`self.MaxSpeedAttcak`))))

(fn `GetStatByLevel`
  (params (Base :type "Float (double-precision)") (IncByLevel :type "Float (double-precision)") (Max :type "Float (double-precision)"))
  (returns (Stat :type "Float (double-precision)"))
  (locals (L_temp :type "Float (double-precision)"))
  (set `local.L_temp` Base)
  (for _ (range 2 (+ (`self.Level`) 1))
    (set `local.L_temp` (* (`local.L_temp`) (`local.IncByLevel`))))
  (return (`KismetMathLibrary.SelectFloat` (`local.L_temp`) (`KismetMathLibrary.FMin` (`local.L_temp`) (`local.Max`)) (== (`local.Max`) -1.0))))

(fn `UpdateLevel`
  (locals (L_OldLevel :type Integer))
  (set `local.L_OldLevel` (`self.Level`))
  (set `self.Level` (`self.GetLevelByExp` (`self.Exp`)))
  (if (< (`local.L_OldLevel`) (`self.Level`))
    (`self.ED_LevelUp`)))